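; CEO is an enemy pawn that chases the VR player and dies after taking enough sword hits.
; PawnSensing spots a MotionControllerPawn and AIMoveTo walks the CEO toward it to a close acceptance radius.
; Each capsule overlap with a sword_Blueprint actor subtracts one point from Health2, and the actor destroys itself when health reaches zero.
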(event `self.PawnSensing.OnSeePawn`
  (params (Pawn :type "Pawn Object Reference"))
  (bind _asmotion_controller_pawn (cast `/Game/VirtualRealityBP/Blueprints/MotionControllerPawn` Pawn))
  (`|AIMoveTo` self (0.0 0.0 0.0) _asmotion_controller_pawn 6.0))

(event `self.CapsuleComponent.OnComponentBeginOverlap`
  (params (OverlappedComponent :type "PrimitiveComponent Object Reference") (OtherActor :type "Actor Object Reference") (OtherComp :type "PrimitiveComponent Object Reference") (OtherBodyIndex :type Integer) (bFromSweep :type Boolean) (SweepResult :type "HitResult Structure (by ref)"))
  (cast `/Game/Unreal-Models/object/sword_Blueprint` OtherActor)
  (`KismetSystemLibrary.PrintString` "")
  (bind _output_get (set `self.Health2` (- (`self.Health2`) 1.0)))
  (if (<= _output_get 0.0)
    (`self.K2_DestroyActor`)))

(fn `UserConstructionScript`)